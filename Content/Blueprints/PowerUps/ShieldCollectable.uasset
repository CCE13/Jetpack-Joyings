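; Shield power-up pickup that grants the collecting player a shield.
; On Collected it plays a pickup sound, then resets the timer of the player's existing shield if one is held.
; Otherwise it spawns a Shield, attaches it to the player, stores it in HoldingShield and shows the shield indicator on the first player's HUD.
; The pickup destroys itself once either path completes.
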(event `/Game/Blueprints/Interface/ICollectable.Collected`
  (params (Player :type "/Game/ThirdPersonBP/Blueprints/ThirdPersonCharacter Object Reference"))
  (`GameplayStatics.PlaySoundAtLocation` "/Game/Sound/powerup_collect.powerup_collect" (`self.K2_GetActorLocation`) (struct) 0.6 1.0 0.0 null null null)
  (if (`KismetSystemLibrary.IsValid` (`/Game/ThirdPersonBP/Blueprints/ThirdPersonCharacter.HoldingShield` Player))
    (bind _asshield (cast `/Game/Blueprints/PowerUps/Shield` (`/Game/ThirdPersonBP/Blueprints/ThirdPersonCharacter.HoldingShield` Player)))
    (`/Game/Blueprints/PowerUps/Shield.ResetTimer` _asshield)
    (else
      (bind _returnvalue (`|SpawnActorFromClass` "/Game/Blueprints/PowerUps/Shield.Shield_C" (`self.GetTransform` Player) "Undefined" "OverrideRootScale" null null))
      (set `/Game/ThirdPersonBP/Blueprints/ThirdPersonCharacter.HoldingShield` _returnvalue Player)
      (`self.K2_AttachToActor` _returnvalue Player "None" "KeepWorld" "KeepWorld" "KeepWorld" true)
      (bind _asplayer_hud (cast `/Game/Blueprints/UI/PlayerHUD` (`PlayerController.GetHUD` (`GameplayStatics.GetPlayerController` 0))))
      (`/Game/Blueprints/UI/GameplayUI.Set Shield Active` (`/Game/Blueprints/UI/PlayerHUD.Gameplay UI Screen` _asplayer_hud) "Visible")))
  (`self.K2_DestroyActor`))

(fn `UserConstructionScript`)