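; Magnetor is a timed coin-magnet power-up actor that pulls nearby coins toward itself.
; Each tick it eases every Coins actor overlapping its Magnet component toward its location with an ease-in blend.
; Its timer drops by a fixed step per tick, so duration depends on frame rate, and ResetTimer restores the starting value.
; On expiry it destroys itself and hides the magnet indicator on the player HUD.
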(event `self.ReceiveBeginPlay`
  (set `self.Startting Timer` (`self.Timer`)))

(event `self.ReceiveTick`
  (params (DeltaSeconds :type "Float (single-precision)"))
  (bind _returnvalue (`self.Countdown`))
  (if _returnvalue
    (`self.K2_DestroyActor`)
    (bind _asplayer_hud (cast `/Game/Blueprints/UI/PlayerHUD` (`PlayerController.GetHUD` (`GameplayStatics.GetPlayerController` 0))))
    (`/Game/Blueprints/UI/GameplayUI.SetMagnetActive` (`/Game/Blueprints/UI/PlayerHUD.Gameplay UI Screen` _asplayer_hud) "Hidden")
    (else
      (for _array_element (`PrimitiveComponent.GetOverlappingActors` (`self.Magnet`) "/Game/Blueprints/Coins/Coins.Coins_C")
        (cast `/Game/Blueprints/Coins/Coins` _array_element)
        (`self.Attract To Player` _array_element)))))

(fn `Attract To Player`
  (params (Object :type "Object Object Reference"))
  (bind _ascoins (cast `/Game/Blueprints/Coins/Coins` Object))
  (`self.K2_SetActorLocation` _ascoins (`|EaseFunction` "EaseIn" 0.4 (`SceneComponent.K2_GetComponentLocation` (`Actor.RootComponent` _ascoins)) (`self.K2_GetActorLocation`)) false false))

(fn `Countdown`
  (returns (ReturnValue :type Boolean))
  (bind _output_get (set `self.Timer` (- (`self.Timer`) 0.05)))
  (return (<= _output_get 0.0)))

(fn `ResetTimer`
  (set `self.Timer` (`self.Startting Timer`)))

(fn `UserConstructionScript`)