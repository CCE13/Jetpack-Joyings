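; Pivot actor for a long laser that tracks the player's position while staying at its configured height.
; Every tick it moves to the third-person character's rounded X and exact Y, then sets the child LongLaser's beam width range.
; While ShootLaser is true, it first changes the laser's sphere material color; following runs whether or not it is shooting.
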(event `self.ReceiveTick`
  (params (DeltaSeconds :type "Float (single-precision)"))
  (if (`self.ShootLaser`)
    (bind _aslong_laser (cast `/Game/Blueprints/Lasers/LongLaser` (`ChildActorComponent.ChildActor` (`self.Laser`))))
    (`/Game/Blueprints/Lasers/Laser.ChangeSphereMaterialColor` _aslong_laser))
  (`self.FollowPlayer`))

(fn `FollowPlayer`
  (bind _asthird_person_character (cast `/Game/ThirdPersonBP/Blueprints/ThirdPersonCharacter` (`GameplayStatics.GetPlayerPawn` 0)))
  (bind (_returnvalue_x _returnvalue_y) (`KismetMathLibrary.BreakVector` (`SceneComponent.K2_GetComponentLocation` (`Actor.RootComponent` _asthird_person_character))))
  (`self.K2_SetActorLocation` self (`KismetMathLibrary.MakeVector` (`KismetMathLibrary.Conv_IntToDouble` (`KismetMathLibrary.Round` _returnvalue_x)) _returnvalue_y (`self.ZPos`)) false false)
  (bind _aslong_laser (cast `/Game/Blueprints/Lasers/LongLaser` (`ChildActorComponent.ChildActor` (`self.Laser`))))
  (`/Game/Blueprints/Lasers/Laser.SetBeamWidth` _aslong_laser 0.0 1.0))

(fn `UserConstructionScript`
  (`parent.UserConstructionScript`))