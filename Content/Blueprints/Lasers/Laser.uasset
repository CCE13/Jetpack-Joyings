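; Laser hazard actor placed on a tile: a beam between two spheres with a death box between them and hurt sounds on kill.
; LaserSetup randomizes length and pitch, then attaches it to the tile as either a static yellow beam or a red rotating one.
; Rotating lasers hang from a spawned LaserPivot that Tick turns by global time dilation, without delta time.
; It destroys itself through the game mode's LaserSpawned binding.
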(event `self.ReceiveBeginPlay`
  (bind _asthird_person_game_mode (cast `/Game/ThirdPersonBP/Blueprints/ThirdPersonGameMode` (`GameplayStatics.GetGameMode`)))
  (add `/Game/ThirdPersonBP/Blueprints/ThirdPersonGameMode.LaserSpawned` _asthird_person_game_mode (delegate `Deactivate`)))

(event `Deactivate`
  (`self.K2_DestroyActor`))

(event `self.ReceiveTick`
  (params (DeltaSeconds :type "Float (single-precision)"))
  (bind _rotator (`self.Rotator`))
  (if (`self.Can Rotate`)
    (`/Engine/EditorBlueprintResources/StandardMacros.IsValid` _rotator
      (:`Is Valid`
        (`self.K2_AddActorWorldRotation` _rotator (`KismetMathLibrary.MakeRotator` 0.0 (* (`GameplayStatics.GetGlobalTimeDilation`) 2.5)) false false)
        (`FXSystemComponent.SetVectorParameter` (`self.Laser`) "LaserEnd" (`SceneComponent.RelativeLocation` (`self.Sphere1`)))))))

(event `/Game/Blueprints/Interface/IKillable.OnKill`
  (`GameplayStatics.PlaySound2D` "/Game/Sound/Electorcuted.Electorcuted" 1.0 1.0 0.0 null null)
  (`GameplayStatics.PlaySound2D` "/Game/Sound/player_hurt_2.player_hurt_2" 1.0 1.0 0.0 null null))

(fn `ChangeSphereMaterialColor`
  (`MeshComponent.SetVectorParameterValueOnMaterials` (`self.Sphere1`) "Base Color" (1.0 0.0 0.0))
  (`MeshComponent.SetVectorParameterValueOnMaterials` (`self.Sphere`) "Base Color" (1.0 0.0 0.0)))

(fn `Laser Setup`
  (params (Tile :type "/Game/Blueprints/MasterTile Object Reference"))
  (bind (_returnvalue_x _returnvalue_y _returnvalue_z) (`KismetMathLibrary.BreakVector` (`SceneComponent.K2_GetComponentLocation` (`self.Sphere`))))
  (bind (_returnvalue_x_2 _returnvalue_y_2 _returnvalue_z_2) (`KismetMathLibrary.BreakVector` (`SceneComponent.K2_GetComponentLocation` (`/Game/Blueprints/MasterTile.Middle` Tile))))
  (`SceneComponent.K2_SetRelativeLocation` (`self.Sphere1`) (`KismetMathLibrary.MakeVector` (`KismetMathLibrary.RandomFloatInRange` 35.0 45.0)) false false)
  (`self.SetDeathBoxWidthAndLocation`)
  (if (>= _returnvalue_z _returnvalue_z_2)
    (`SceneComponent.K2_SetWorldRotation` (`self.Sphere`) (`KismetMathLibrary.MakeRotator` 0.0 (`KismetMathLibrary.RandomFloatInRange` 180.0 360.0)) false false)
    (else
      (`SceneComponent.K2_SetWorldRotation` (`self.Sphere`) (`KismetMathLibrary.MakeRotator` 0.0 (`KismetMathLibrary.RandomFloatInRange` 0.0 180.0)) false false)))
  (`FXSystemComponent.SetVectorParameter` (`self.Laser`) "LaserEnd" (`SceneComponent.RelativeLocation` (`self.Sphere1`)))
  (bind _output_get (set `self.Can Rotate` (`KismetMathLibrary.RandomBool`)))
  (if _output_get
    (`FXSystemComponent.SetColorParameter` (`self.Laser`) "Color" (struct :`R` 1.0 :`A` 1.0))
    (bind _returnvalue (`|SpawnActorFromClass` "/Game/Blueprints/Lasers/LaserPivot.LaserPivot_C" (`SceneComponent.K2_GetComponentToWorld` (`self.Death`)) "Undefined" "OverrideRootScale" null null))
    (bind _output_get_2 (set `self.Rotator` _returnvalue))
    (`self.K2_AttachToActor` _output_get_2 "None" "KeepWorld" "KeepWorld" "KeepWorld")
    (`self.K2_AttachToActor` (`self.Rotator`) Tile "None" "KeepWorld" "KeepWorld" "KeepWorld" true)
    (else
      (`FXSystemComponent.SetColorParameter` (`self.Laser`) "Color" (struct :`R` 0.982251 :`G` 1.0 :`A` 1.0))
      (`self.K2_AttachToActor` Tile "None" "KeepWorld" "KeepWorld" "KeepWorld"))))

(fn `SetBeamWidth`
  (params (MinimumWidth :type "Float (double-precision)") (MaximumWidth :type "Float (double-precision)"))
  (`FXSystemComponent.SetFloatParameter` (`self.Laser`) "MaximumBeamWidth" MaximumWidth)
  (`FXSystemComponent.SetFloatParameter` (`self.Laser`) "MinimumBeamWidth" MinimumWidth))

(fn `SetDeathBoxWidthAndLocation`
  (bind _death (`self.Death`))
  (bind _returnvalue_x (`KismetMathLibrary.BreakVector` (`SceneComponent.K2_GetComponentLocation` (`self.Sphere`))))
  (bind _returnvalue_x_2 (`KismetMathLibrary.BreakVector` (`SceneComponent.K2_GetComponentLocation` (`self.Sphere1`))))
  (bind (_boxextent_x _boxextent_y _boxextent_z) (`KismetMathLibrary.BreakVector` (`BoxComponent.BoxExtent` _death)))
  (bind _relativelocation_x (`KismetMathLibrary.BreakVector` (`SceneComponent.RelativeLocation` (`self.Sphere`))))
  (bind _relativelocation_x_2 (`KismetMathLibrary.BreakVector` (`SceneComponent.RelativeLocation` (`self.Sphere1`))))
  (`SceneComponent.K2_SetRelativeLocation` (`self.Death`) (`KismetMathLibrary.MakeVector` (/ (- _relativelocation_x_2 _relativelocation_x) 2.0)) false false)
  (`BoxComponent.SetBoxExtent` _death (`KismetMathLibrary.MakeVector` (/ (- _returnvalue_x_2 _returnvalue_x) 2.0) _boxextent_y _boxextent_z) true))

(fn `UserConstructionScript`
  (`self.SetBeamWidth` 2.0 4.0))