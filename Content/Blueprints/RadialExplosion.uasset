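; RadialExplosion is an actor that sets off a physics explosion when the player character's StartGame event fires.
; On BeginPlay it deactivates its Explosion component and binds Explode to that event on the ThirdPersonCharacter.
; Explode enables physics simulation on the static mesh actors in ItemsToActivatePhysics, then fires the RadialForce impulse and activates Explosion, so props stay static until the blast.
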(event `self.ReceiveBeginPlay`
  (`ActorComponent.Deactivate` (`self.Explosion`))
  (bind _asthird_person_character (cast `/Game/ThirdPersonBP/Blueprints/ThirdPersonCharacter` (`GameplayStatics.GetPlayerPawn` 0)))
  (add `/Game/ThirdPersonBP/Blueprints/ThirdPersonCharacter.StartGame` _asthird_person_character (delegate `Explode`)))

(event `self.ReceiveTick`
  (params (DeltaSeconds :type "Float (single-precision)")))

(event `Explode`
  (for _array_element (`self.ItemsToActivatePhysics`)
    (bind _asstatic_mesh_actor (cast `StaticMeshActor` _array_element))
    (`PrimitiveComponent.SetSimulatePhysics` (`StaticMeshActor.StaticMeshComponent` _asstatic_mesh_actor) true))
  (`RadialForceComponent.FireImpulse` (`self.RadialForce`))
  (`ActorComponent.Activate` (`self.Explosion`) false))

(fn `UserConstructionScript`)