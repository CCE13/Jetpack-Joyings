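; Collectible coin actor that spins while on screen and adds to the player's coin count when collected.
; Tick uses a RotateOnce gate to play a yaw timeline when the coin passes a viewport check, which only tests the right screen edge with a margin.
; Collected calls AddCoins on the ThirdPersonGameMode, plays a random sound at the coin's location and destroys the actor.
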(event `self.ReceiveTick`
  (params (DeltaSeconds :type "Float (single-precision)"))
  (if (not (`self.RotateOnce`))
    (bind _returnvalue (`self.Is Coin In Viewport?`))
    (if _returnvalue
      (set `self.RotateOnce` true)
      (bind (_direction _rotation) (`Timeline|Rotate`)
        (:`Update`
          _)
        (:`Finished`
          (set `self.RotateOnce` false)))
      (`self.K2_SetActorRotation` (`KismetMathLibrary.MakeRotator` 0.0 0.0 _rotation)))))

(event `/Game/Blueprints/Interface/ICollectable.Collected`
  (params (Player :type "/Game/ThirdPersonBP/Blueprints/ThirdPersonCharacter Object Reference"))
  ;[1 1 1] Plays a random sound on collected
  (bind _asthird_person_game_mode (cast `/Game/ThirdPersonBP/Blueprints/ThirdPersonGameMode` (`GameplayStatics.GetGameMode`)))
  (`/Game/ThirdPersonBP/Blueprints/ThirdPersonGameMode.Add Coins` _asthird_person_game_mode)
  (`GameplayStatics.PlaySoundAtLocation` (`KismetArrayLibrary.Array_Random` (`self.Sound`)) (`self.K2_GetActorLocation`) (struct) 1.0 1.0 0.0 null null null)
  (`self.K2_DestroyActor`))

(fn `Is Coin In Viewport?`
  (returns (ReturnValue :type Boolean))
  (bind _returnvalue_x (`KismetMathLibrary.BreakVector2D` (`WidgetLayoutLibrary.GetViewportSize`)))
  (return (> _returnvalue_x (+ (`KismetMathLibrary.BreakVector2D` (`GameplayStatics.ProjectWorldToScreen` (`GameplayStatics.GetPlayerController` 0) (`SceneComponent.K2_GetComponentLocation` (`self.Coin`)))) 100.0))))

(fn `UserConstructionScript`
  (`parent.UserConstructionScript`))