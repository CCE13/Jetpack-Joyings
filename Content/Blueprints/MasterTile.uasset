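; MasterTile is a level tile actor that varies its look and population on spawn and removes itself after the player reaches it.
; On BeginPlay it picks a random background mesh and, on a coin flip, spawns a few Scientists at SpawnMinX.
; A ThirdPersonCharacter overlapping its Box arms a per-frame countdown, halted while PlayerHUD is paused.
; At zero it destroys attached actors two levels deep, then itself.
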(event `self.ReceiveBeginPlay`
  (`StaticMeshComponent.SetStaticMesh` (`self.StaticMesh`) (`KismetArrayLibrary.Array_Random` (`self.BackgroundMeshes`)))
  (if (`KismetMathLibrary.RandomBool`)
    (for _ (range (+ (`KismetMathLibrary.RandomIntegerInRange` 0 3) 1))
      (`|SpawnActorFromClass` "/Game/Blueprints/AI/Scientist.Scientist_C" (`KismetMathLibrary.MakeTransform` (`SceneComponent.K2_GetComponentLocation` (`self.Spawn Min X`))) "AdjustIfPossibleButDontSpawnIfColliding" "OverrideRootScale" null null))))

(event `self.ReceiveTick`
  (params (DeltaSeconds :type "Float (single-precision)"))
  (bind _asplayer_hud (cast `/Game/Blueprints/UI/PlayerHUD` (`PlayerController.GetHUD` (`GameplayStatics.GetPlayerController` 0))))
  (if (`/Game/Blueprints/UI/PlayerHUD.IsPaused` _asplayer_hud)
    _
    (elif (`self.CanDie`)
      (set `self.Timer` (- (`self.Timer`) 0.01))
      (if (<= (`self.Timer`) 0.0)
        (for _array_element (`self.GetAttachedActors` false)
          (bind _outactors (`self.GetAttachedActors` _array_element true))
          (if (> (`KismetArrayLibrary.Array_Length` _outactors) 0)
            (for _array_element_2 _outactors
              (`self.K2_DestroyActor` _array_element_2)))
          (`self.K2_DestroyActor` _array_element))
        (`self.K2_DestroyActor`)))))

(event `self.Box.OnComponentBeginOverlap`
  (params (OverlappedComponent :type "PrimitiveComponent Object Reference") (OtherActor :type "Actor Object Reference") (OtherComp :type "PrimitiveComponent Object Reference") (OtherBodyIndex :type Integer) (bFromSweep :type Boolean) (SweepResult :type "HitResult Structure (by ref)"))
  (cast `/Game/ThirdPersonBP/Blueprints/ThirdPersonCharacter` OtherActor)
  (set `self.CanDie` true))

(fn `UserConstructionScript`)