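; Camera actor Blueprint that follows the player along the X axis once the game has started.
; Each Tick it casts the player pawn to ThirdPersonCharacter and checks its GameStarted flag.
; When set, it moves its Camera component to the character's X position while keeping its own Y and Z, as in a side-scroller.
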(event `self.ReceiveActorBeginOverlap`
  (params (OtherActor :type "Actor Object Reference")))

(event `self.ReceiveTick`
  (params (DeltaSeconds :type "Float (single-precision)"))
  (bind _asthird_person_character (cast `/Game/ThirdPersonBP/Blueprints/ThirdPersonCharacter` (`GameplayStatics.GetPlayerPawn` 0)))
  (if (`/Game/ThirdPersonBP/Blueprints/ThirdPersonCharacter.GameStarted` _asthird_person_character)
    (`SceneComponent.K2_SetWorldLocation` (`self.Camera`) (`KismetMathLibrary.MakeVector` (.x (`SceneComponent.K2_GetComponentLocation` (`Actor.RootComponent` _asthird_person_character))) (.y (`SceneComponent.K2_GetComponentLocation` (`self.Camera`))) (.z (`SceneComponent.K2_GetComponentLocation` (`self.Camera`)))) false false)))

(fn `UserConstructionScript`)